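; BP_SenseBudgetWalker is an actor that moves itself continuously along a fixed figure-eight path centred on the world origin.
; Each Tick derives an absolute location from game time, using two degree-based sine waves with Y at twice the frequency of X and a constant height.
; It teleports there without sweeping, so motion depends only on the clock, not on collision or its placed position.
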(event EventBeginPlay)

(event Collision|EventActorBeginOverlap
  (params (OtherActor :type Actor%20Object%20Reference)))

(event EventTick
  (params (DeltaSeconds :type Float%20%28single-precision%29))
  (bind _returnvalue (Utilities|Time|GetGameTimeinSeconds))
  (Transformation|SetActorLocation (Math|Vector|MakeVector (* (Math|Trig|Sin(Degrees) (* _returnvalue (Math|Float|MakeLiteralFloat 8.0))) (Math|Float|MakeLiteralFloat 5.2e+03)) (* (Math|Trig|Sin(Degrees) (* _returnvalue (Math|Float|MakeLiteralFloat 16.0))) (Math|Float|MakeLiteralFloat 3e+03)) 6e+01) false true))

(fn ConstructionScript)