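; BP_SenseGuardPatrol is a guard actor that visually shows its current SenseBudget tier through its color.
; On BeginPlay it applies a uniform scale from GuardScale.
; Every Tick it reads the tier display color from SenseBudget and pushes it as the TierColor vector parameter to the Body and Head materials.
; The graph itself contains no patrol movement or sensing logic.
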(event EventBeginPlay
  (bind _guardscale (Variables|Default|GetGuardScale))
  (Transformation|SetActorScale3D (Math|Vector|MakeVector _guardscale _guardscale _guardscale)))

(event Collision|EventActorBeginOverlap
  (params (OtherActor :type Actor%20Object%20Reference)))

(event EventTick
  (params (DeltaSeconds :type Float%20%28single-precision%29))
  (bind _sensebudget (Variables|Default|GetSenseBudget))
  (bind _returnvalue (Class|SenseBudgetComponent|GetTierDisplayColor _sensebudget))
  (bind (_r _g _b) (Utilities|Struct|BreakLinearColor _returnvalue))
  (bind _returnvalue_2 (Math|Vector|MakeVector _r _g _b))
  (Rendering|Material|SetVectorParameterValueonMaterials (Variables|Default|GetBody) "TierColor" _returnvalue_2)
  (Rendering|Material|SetVectorParameterValueonMaterials (Variables|Default|GetHead) "TierColor" _returnvalue_2))

(fn ConstructionScript)