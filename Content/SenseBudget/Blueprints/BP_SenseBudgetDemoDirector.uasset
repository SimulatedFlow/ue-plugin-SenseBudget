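; Demo director for SenseBudget that populates the level with 96 sense guards on BeginPlay.
; Nested loops lay out a 12 by 8 grid centered on the world origin, with random position jitter and yaw per guard.
; The flattened grid index modulo 6 picks the class, giving a fixed 1:2:3 mix of Elite, Civilian and Patrol guards, always spawned regardless of collision.
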(event EventBeginPlay
  (for _index (range 0 11)
    (for _index_2 (range 0 7)
      (if (== (Math|Integer|%(Integer) (+ (* _index (Class|KismetSystemLibrary|MakeLiteralInteger 8)) _index_2) 6) (Class|KismetSystemLibrary|MakeLiteralInteger))
        (Game|SpawnActorfromClass "/SenseBudget/SenseBudget/Blueprints/BP_SenseGuardElite.BP_SenseGuardElite_C" (Math|Transform|MakeTransform (Math|Vector|MakeVector (+ (- (* _index (Math|Float|MakeLiteralFloat 9.5e+02)) (Math|Float|MakeLiteralFloat 5225.0)) (- (Math|Random|RandomFloatinRange 0.0 3e+02) (Math|Float|MakeLiteralFloat 1.5e+02))) (+ (- (* _index_2 (Math|Float|MakeLiteralFloat 9e+02)) (Math|Float|MakeLiteralFloat 3.15e+03)) (- (Math|Random|RandomFloatinRange 0.0 3e+02) (Math|Float|MakeLiteralFloat 1.5e+02))) 0.0) (Math|Rotator|MakeRotator 0.0 0.0 (Math|Random|RandomFloatinRange 0.0 3.6e+02))) "AlwaysSpawn" "MultiplyWithRoot" 0 0)
        (elif (< (Math|Integer|%(Integer) (+ (* _index (Class|KismetSystemLibrary|MakeLiteralInteger 8)) _index_2) 6) (Class|KismetSystemLibrary|MakeLiteralInteger 3))
          (Game|SpawnActorfromClass "/SenseBudget/SenseBudget/Blueprints/BP_SenseGuardCivilian.BP_SenseGuardCivilian_C" (Math|Transform|MakeTransform (Math|Vector|MakeVector (+ (- (* _index (Math|Float|MakeLiteralFloat 9.5e+02)) (Math|Float|MakeLiteralFloat 5225.0)) (- (Math|Random|RandomFloatinRange 0.0 3e+02) (Math|Float|MakeLiteralFloat 1.5e+02))) (+ (- (* _index_2 (Math|Float|MakeLiteralFloat 9e+02)) (Math|Float|MakeLiteralFloat 3.15e+03)) (- (Math|Random|RandomFloatinRange 0.0 3e+02) (Math|Float|MakeLiteralFloat 1.5e+02))) 0.0) (Math|Rotator|MakeRotator 0.0 0.0 (Math|Random|RandomFloatinRange 0.0 3.6e+02))) "AlwaysSpawn" "MultiplyWithRoot" 0 0)
          (else
            (Game|SpawnActorfromClass "/SenseBudget/SenseBudget/Blueprints/BP_SenseGuardPatrol.BP_SenseGuardPatrol_C" (Math|Transform|MakeTransform (Math|Vector|MakeVector (+ (- (* _index (Math|Float|MakeLiteralFloat 9.5e+02)) (Math|Float|MakeLiteralFloat 5225.0)) (- (Math|Random|RandomFloatinRange 0.0 3e+02) (Math|Float|MakeLiteralFloat 1.5e+02))) (+ (- (* _index_2 (Math|Float|MakeLiteralFloat 9e+02)) (Math|Float|MakeLiteralFloat 3.15e+03)) (- (Math|Random|RandomFloatinRange 0.0 3e+02) (Math|Float|MakeLiteralFloat 1.5e+02))) 0.0) (Math|Rotator|MakeRotator 0.0 0.0 (Math|Random|RandomFloatinRange 0.0 3.6e+02))) "AlwaysSpawn" "MultiplyWithRoot" 0 0)))))))

(event Collision|EventActorBeginOverlap
  (params (OtherActor :type Actor%20Object%20Reference)))

(event EventTick
  (params (DeltaSeconds :type Float%20%28single-precision%29)))

(fn ConstructionScript)